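; Horror Engine game instance holding session state such as save slot, player and inventory caches, pickup counts and elapsed time.
; Its RsetVar event tells placed Battery, Key and gift box actors to reset when their counts are nonzero, always calling the first actor found, repeated per battery up to three.
; It then restores caches and slot name from start values and clears flags, counters and timer.
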(event `RsetVar`
  (`|ExecutionSequence`
    (:`then_0`
      (if (not (== (`self.Num_Bettary`) 0))
        (bind _asbattery (castclass `/Game/HorrorEngine/Blueprints/UsableAssets/Inventory/Battery` "/Game/HorrorEngine/Blueprints/UsableAssets/Inventory/Battery.Battery_C"))
        (bind _outactors (`GameplayStatics.GetAllActorsOfClass` _asbattery))
        (if (== (`self.Num_Bettary`) 3)
          (bind _output (`|GetArrayItem` _outactors))
          (`/Game/HorrorEngine/Blueprints/UsableAssets/Inventory/Battery.BatteryReset` _output)
          (`/Game/HorrorEngine/Blueprints/UsableAssets/Inventory/Battery.BatteryReset` _output)
          (`/Game/HorrorEngine/Blueprints/UsableAssets/Inventory/Battery.BatteryReset` _output)
          (elif (== (`self.Num_Bettary`) 2)
            (`/Game/HorrorEngine/Blueprints/UsableAssets/Inventory/Battery.BatteryReset` _output)
            (`/Game/HorrorEngine/Blueprints/UsableAssets/Inventory/Battery.BatteryReset` _output)
            (elif (== (`self.Num_Bettary`) 1)
              (`/Game/HorrorEngine/Blueprints/UsableAssets/Inventory/Battery.BatteryReset` _output)
              (`KismetSystemLibrary.PrintString` "베터리1초기화"))))))
    (:`then_1`
      (if (not (== (`self.Num_Key`) 0))
        (bind _askey (castclass `/Game/HorrorEngine/Blueprints/UsableAssets/Inventory/Key` "/Game/HorrorEngine/Blueprints/UsableAssets/Inventory/Key.Key_C"))
        (bind _outactors_2 (`GameplayStatics.GetAllActorsOfClass` _askey))
        (`/Game/HorrorEngine/Blueprints/UsableAssets/Inventory/Key.KeyReset` (`|GetArrayItem` _outactors_2))))
    (:`then_2`
      (if (not (== (`self.Num_GiftBox`) 0))
        (bind _asbp_gift_box (castclass `/Game/KJH/BP/BP_GiftBox` "/Game/KJH/BP/BP_GiftBox.BP_GiftBox_C"))
        (bind _outactors_3 (`GameplayStatics.GetAllActorsOfClass` _asbp_gift_box))
        (`/Game/KJH/BP/BP_GiftBox.GiftBoxReset` (`|GetArrayItem` _outactors_3))))
    (:`then_3`
      (set `self.Loading` false)
      (set `self.NewLevel` false)
      (set `self.PlayerCache` (`self.PlayerCache_Start`))
      (set `self.InventoryCache` (`self.InventoryCache_Start`))
      (set `self.SlotName` (`self.SlotName_Start`))
      (set `self.Num_Bettary` 0)
      (set `self.Num_Key` 0)
      (set `self.Num_GiftBox` 0)
      (set `self.ElapsedTime` 0.0))))