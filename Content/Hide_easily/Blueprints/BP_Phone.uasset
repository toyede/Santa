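; Phone hiding place, a single-door child of a parent hiding-spot Blueprint, which the player can enter and leave.
; The construction script removes the inherited left-door components, and a timeline swings the right door, with length and curve set by hide speed.
; Hide and Unhide sequence door movement and player movement with speed-based delays, driving the PlayerController through BI_HideEasilyControl for input, optional rotation and prompt messages.
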(event `self.OpenDoors`
  ;[1 1 1] OPEN/CLOSE DORS  overwrite
  (bind (_direction _track_0) (`Timeline|New Open/Close Doors` :!label _label)
    (:`Update`
      (`SceneComponent.K2_SetRelativeRotation` (`self.RightDoorRoot`) (`KismetMathLibrary.RLerp` (struct :`Pitch` 90.0 :`Yaw` 180.0 :`Roll` 180.0) (struct :`Pitch` 90.0 :`Yaw` 180.0 :`Roll` 90.0) _track_0 true) false false))))

(event `self.CloseDoors`
  ;[1 1 1] OPEN/CLOSE DORS  overwrite
  (goto _label :!via `Reverse`))

(event `self.Hide`
  (params (Pawn :type "Actor Object Reference") (PlayerController :type "PlayerController Object Reference"))
  (bind _asbi_hide_easily_control (cast `/Game/Hide_easily/Blueprints/GameModeAndController/BI_HideEasilyControl` PlayerController :!pure true))
  (bind _value (`BlueprintMapLibrary.Map_Find` (`self.Delays`) (`self.HideSpeed`)))
  (bind _returnvalue (`SceneComponent.K2_GetComponentLocation` (`Actor.RootComponent` Pawn)))
  (`/Game/Hide_easily/Blueprints/GameModeAndController/BI_HideEasilyControl.BI Update Hiding` _asbi_hide_easily_control true)
  (`/Game/Hide_easily/Blueprints/GameModeAndController/BI_HideEasilyControl.BI Disable Player Input` _asbi_hide_easily_control)
  (set `self.Hiding` true)
  (`self.Server_Hide_Message` _asbi_hide_easily_control)
  ;[1 1 1] Rotate
  (if (`self.RotateBeforeHide`)
    (`/Game/Hide_easily/Blueprints/GameModeAndController/BI_HideEasilyControl.BI Rotate To Face Doors` _asbi_hide_easily_control Pawn _returnvalue (`SceneComponent.K2_GetComponentLocation` (`self.Location_In`)))
    (`KismetSystemLibrary.Delay` 0.2))
  (`self.OpenDoors`)
  (`KismetSystemLibrary.Delay` (`BlueprintMapLibrary.Map_Find` (`self.Delays`) (`self.HideSpeed`)))
  (`KismetSystemLibrary.Delay` 0.1)
  (`/Game/Hide_easily/Blueprints/GameModeAndController/BI_HideEasilyControl.BI Player Go In` _asbi_hide_easily_control _returnvalue (`SceneComponent.K2_GetComponentLocation` (`self.Location_In`)) Pawn (`self.HideSpeed`) (`self.RotateWhenHide`))
  (`KismetSystemLibrary.Delay` _value)
  (`self.CloseDoors`)
  (`KismetSystemLibrary.Delay` (+ _value 0.5)) ; wait until you get inside
  (`/Game/Hide_easily/Blueprints/GameModeAndController/BI_HideEasilyControl.BI Add Hiding Place` _asbi_hide_easily_control self)
  (`self.Server_Show_Message` _asbi_hide_easily_control) ; enable unhide
  (set `self.Hiding` false)
  (`/Game/Hide_easily/Blueprints/GameModeAndController/BI_HideEasilyControl.BI Update Hiding` _asbi_hide_easily_control false))

(event `self.Unhide`
  (params (Pawn :type "Actor Object Reference") (`Player Controller` :type "/Game/Hide_easily/Blueprints/GameModeAndController/BI_HideEasilyControl Interface"))
  (`/Game/Hide_easily/Blueprints/GameModeAndController/BI_HideEasilyControl.BI Update Hiding` `Player Controller` true)
  (`self.Server_Hide_Message` `Player Controller`)
  (set `self.Unhiding` true) ; to know when you start leaving the closet
  (`self.OpenDoors`)
  (`KismetSystemLibrary.Delay` (`BlueprintMapLibrary.Map_Find` (`self.Delays`) (`self.HideSpeed`)))
  (`/Game/Hide_easily/Blueprints/GameModeAndController/BI_HideEasilyControl.BI Player Go Out` `Player Controller` (`SceneComponent.K2_GetComponentLocation` (`Actor.RootComponent` Pawn)) (`SceneComponent.K2_GetComponentLocation` (`self.Location_Out`)) Pawn (`self.HideSpeed`))
  (`KismetSystemLibrary.Delay` (+ (`BlueprintMapLibrary.Map_Find` (`self.Delays`) (`self.HideSpeed`)) 0.1))
  (`self.CloseDoors`)
  (`KismetSystemLibrary.Delay` 0.8)
  (set `self.Unhiding` false) ; you left the closet
  (`/Game/Hide_easily/Blueprints/GameModeAndController/BI_HideEasilyControl.BI Update Hiding` `Player Controller` false))

(fn `SetHideSpeed`
  (bind _new_open_close_doors (`self.New Open/Close Doors`))
  (bind _hidespeed (`self.HideSpeed`))
  (`TimelineComponent.SetTimelineLength` _new_open_close_doors (select `/Game/Hide_easily/Blueprints/GameModeAndController/E_HideSpeed` _hidespeed :`NewEnumerator0` 0.7 :`NewEnumerator1` 0.5 :!type "Float (single-precision)"))
  (`TimelineComponent.SetFloatCurve` _new_open_close_doors (select `/Game/Hide_easily/Blueprints/GameModeAndController/E_HideSpeed` _hidespeed :`NewEnumerator0` "/Game/Hide_easily/Curves/C_Point7.C_Point7" :`NewEnumerator1` "/Game/Hide_easily/Curves/C_Point5.C_Point5" :!type "CurveFloat Object Reference") "Track_0"))

(fn `UserConstructionScript`
  (`parent.UserConstructionScript`)
  (`ActorComponent.K2_DestroyComponent` (`self.LeftDoorRoot`))
  (`ActorComponent.K2_DestroyComponent` (`self.LeftDoorMesh`))
  (`ActorComponent.K2_DestroyComponent` (`self.LeftDoorknob`)))