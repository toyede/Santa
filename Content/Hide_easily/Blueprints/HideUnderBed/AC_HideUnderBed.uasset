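; Component that plays the hide, idle and unhide animations for a character hiding under a bed.
; Server-named events sequence each transition with fixed delays, using Multicast-named events to play animation assets directly on the mesh.
; Hiding disables movement and loops the idle; unhiding restores the Animation Blueprint and walking.
; It toggles camera control rotation and notifies the hide controller through BI_HideEasilyControl to adjust and re-enable input.
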(event `MulticastUnhideAnimation`
  (params (Mesh :type "SkeletalMeshComponent Object Reference"))
  ;[1 0.5048 0.01547] Under Bed aNIMATIONS
  ;;[1 1 1] Comment
  (`SkeletalMeshComponent.PlayAnimation` Mesh "/Game/Hide_easily/Animations/AS_UnhideBed.AS_UnhideBed" false))

(event `ServerSetAnimationMode`
  (params (Mesh :type "SkeletalMeshComponent Object Reference"))
  ;[1 0.5048 0.01547] Under Bed aNIMATIONS
  ;;[1 1 1] Comment
  (`self.BackToAnimationClass` Mesh))

(event `MulticastRunHideAnimation`
  (params (Mesh :type "SkeletalMeshComponent Object Reference"))
  ;[1 0.5048 0.01547] Under Bed aNIMATIONS
  ;;[1 1 1] Comment
  (`SkeletalMeshComponent.PlayAnimation` Mesh "/Game/Hide_easily/Animations/AS_HideUnderBed.AS_HideUnderBed" false))

(event `BackToAnimationClass`
  (params (Mesh :type "SkeletalMeshComponent Object Reference"))
  ;[1 0.5048 0.01547] Under Bed aNIMATIONS
  ;;[1 1 1] Comment
  (`SkeletalMeshComponent.SetAnimationMode` Mesh "AnimationBlueprint"))

(event `MulticastRunIdleAnimation`
  (params (Mesh :type "SkeletalMeshComponent Object Reference"))
  ;[1 0.5048 0.01547] Under Bed aNIMATIONS
  ;;[1 1 1] Comment
  (`SkeletalMeshComponent.PlayAnimation` Mesh "/Game/Hide_easily/Animations/AS_UnderBedIdle.AS_UnderBedIdle" true))

(event `ChangeControlRotation`
  (params (`Use Pawn Control Rotation` :type Boolean) (Camera :type "CameraComponent Object Reference"))
  ;[1 0.5048 0.01547] Under Bed aNIMATIONS
  (set `CameraComponent.bUsePawnControlRotation` `Use Pawn Control Rotation` Camera))

(event `ServerRunHideAnimation`
  (params (Camera :type "CameraComponent Object Reference") (Mesh :type "SkeletalMeshComponent Object Reference") (Movement :type "CharacterMovementComponent Object Reference") (HideController :type "PlayerController Object Reference"))
  ;[1 0.5048 0.01547] Under Bed aNIMATIONS
  ;;[1 1 1] Hide animation
  (`self.ChangeControlRotation` false Camera)
  (`self.MulticastRunHideAnimation` Mesh)
  (`KismetSystemLibrary.Delay` 0.95)
  (`CharacterMovementComponent.DisableMovement` Movement)
  (`/Game/Hide_easily/Blueprints/GameModeAndController/BI_HideEasilyControl.BI Adjust After Hide` (cast `/Game/Hide_easily/Blueprints/GameModeAndController/BI_HideEasilyControl` HideController :!pure true))
  (`self.MulticastRunIdleAnimation` Mesh)
  (`self.ChangeControlRotation` true Camera))

(event `ServerRunUnhideAnimation`
  (params (HideController :type "PlayerController Object Reference") (Mesh :type "SkeletalMeshComponent Object Reference") (Camera :type "CameraComponent Object Reference") (Movement :type "CharacterMovementComponent Object Reference"))
  (bind _asbi_hide_easily_control (cast `/Game/Hide_easily/Blueprints/GameModeAndController/BI_HideEasilyControl` HideController :!pure true))
  ;[1 0.5048 0.01547] Under Bed aNIMATIONS
  ;;[1 1 1] UnhideAnimation
  (`/Game/Hide_easily/Blueprints/GameModeAndController/BI_HideEasilyControl.BI Adjust After Unhide` _asbi_hide_easily_control)
  (`self.MulticastUnhideAnimation` Mesh)
  (`KismetSystemLibrary.Delay` 0.9)
  (`self.ChangeControlRotation` true Camera)
  (`self.ServerSetAnimationMode` Mesh)
  (`CharacterMovementComponent.SetMovementMode` Movement "MOVE_Walking" 0)
  (`/Game/Hide_easily/Blueprints/GameModeAndController/BI_HideEasilyControl.BI Enable Rotation And Input` _asbi_hide_easily_control))