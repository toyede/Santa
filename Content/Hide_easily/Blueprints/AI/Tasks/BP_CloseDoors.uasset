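; Behavior tree task that makes the AI close the doors of an opened closet.
; When the closet-opened blackboard key is set, it passes the stored location to the AI controller's CloseClosetDoors, clears the search, opened and occupied flags, then succeeds.
; Otherwise it fails; a failed controller cast stops without finishing the task.
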(event `self.ReceiveExecuteAI`
  (params (OwnerController :type "AIController Object Reference") (ControlledPawn :type "Pawn Object Reference"))
  (if (`BTFunctionLibrary.GetBlackboardValueAsBool` (`self.BB_ClosetOpened`))
    (bind _asbp_ai_controller_1 (cast `/Game/Hide_easily/Blueprints/AI/BP_AI-Controller1` OwnerController))
    (`/Game/Hide_easily/Blueprints/AI/BP_AI-Controller1.CloseClosetDoors` _asbp_ai_controller_1 (`BTFunctionLibrary.GetBlackboardValueAsVector` (`self.BB_Location`)))
    (`BTFunctionLibrary.SetBlackboardValueAsBool` (`self.BB_CanSearch`))
    (`BTFunctionLibrary.SetBlackboardValueAsBool` (`self.BB_ClosetOpened`))
    (`BTFunctionLibrary.SetBlackboardValueAsBool` (`self.BB_ClosetOcupied`))
    (`self.FinishExecute` true)
    (else
      (`self.FinishExecute` false))))