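; Behavior Tree task that looks up the current patrol point for an AI character.
; It reads the path index from the Blackboard, takes that entry from the pawn's PatrolPath FinalPoints, and converts it to world space through the path actor's transform.
; The result is written to a Blackboard vector key and the task succeeds.
; A failed cast or invalid path leaves the task without a FinishExecute call.
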(event `self.ReceiveExecuteAI`
  (params (OwnerController :type "AIController Object Reference") (ControlledPawn :type "Pawn Object Reference"))
  (bind _asbp_ai_character (cast `/Game/Hide_easily/Blueprints/AI/BP_AI-Character` ControlledPawn))
  (bind _patrolpath (`/Game/Hide_easily/Blueprints/AI/BP_AI-Character.PatrolPath` _asbp_ai_character)
    (:`then`
      (`BTFunctionLibrary.SetBlackboardValueAsVector` (`self.BB_PathVector`) (`KismetMathLibrary.TransformLocation` (`Actor.GetTransform` _patrolpath) (`|GetArrayItem` (`/Game/Hide_easily/Blueprints/AI/BP_PatrolPathAndClosets.FinalPoints` _patrolpath) (`BTFunctionLibrary.GetBlackboardValueAsInt` (`self.BB_PathIndex`)))))
      (`self.FinishExecute` true))
    (:`else`)))