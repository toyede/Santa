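; Behavior tree task for the AI's attack in Hide_easily, which tells the chased character it is dead and stages a jump scare.
; It calls BIYouAreDead on that character's controller through an interface, passing the kill-player blackboard flag.
; It then teleports the first BP_AICharacter1 found to JumpDistance along the player's view, slightly raised, and calls JumpScare.
; It clears the attack flag and finishes successfully, but any failed cast leaves it unfinished.
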(event `self.ReceiveExecuteAI`
  (params (OwnerController :type "AIController Object Reference") (ControlledPawn :type "Pawn Object Reference"))
  (bind _ascharacter (cast `Character` (`BTFunctionLibrary.GetBlackboardValueAsObject` (`self.BP_ChaseActor`))))
  (bind _asbi_hide_easily_control (cast `/Game/Hide_easily/Blueprints/GameModeAndController/BI_HideEasilyControl` (`Pawn.GetController` _ascharacter)))
  (`/Game/Hide_easily/Blueprints/GameModeAndController/BI_HideEasilyControl.BI You Are Dead` _asbi_hide_easily_control (`BTFunctionLibrary.GetBlackboardValueAsBool` (`self.BP_KillPlayer?`)))
  (bind _asbp_santa_character (cast `/Game/KJH/BP/BP_SantaCharacter` (`GameplayStatics.GetPlayerCharacter` 0)))
  (bind _outactors (`GameplayStatics.GetAllActorsOfClass` "/Game/Hide_easily/Blueprints/AI/BP_AI-Character1.BP_AI-Character1_C"))
  (bind _output_get (set `self.Child` (`|GetArrayItem` _outactors)))
  (`Actor.K2_SetActorLocation` _output_get (+ (+ (`Actor.K2_GetActorLocation` _asbp_santa_character) (* (`KismetMathLibrary.GetForwardVector` (`Controller.GetControlRotation` (`GameplayStatics.GetPlayerController` 0))) (`self.Jump distance`))) (0.0 0.0 100.0)) false false)
  (bind _asbp_ai_character_1 (cast `/Game/Hide_easily/Blueprints/AI/BP_AI-Character1` (`self.Child`)))
  (`/Game/Hide_easily/Blueprints/AI/BP_AI-Character1.JumpScare` _asbp_ai_character_1)
  (`KismetSystemLibrary.PrintString` "You dead")
  (`BTFunctionLibrary.SetBlackboardValueAsBool` (`self.BB_Attack`))
  (`self.FinishExecute` true))