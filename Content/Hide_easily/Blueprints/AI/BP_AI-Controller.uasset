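; AI controller for the hide-and-seek enemy, with tree-to-spawn patrol and audio-backed chase events.
; Perception sets blackboard sight and chase target from the player's hiding, death and distance.
; Tick sends it to the player's room door when the HUD reports noise; helpers check and operate patrol-path closets and beds.
; BeginPlay is empty: setup of HUD reference, patrol, behavior tree and blackboard is disconnected.
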(event `StartPatrol`
  (set `self.bIsPatrolling` true)
  (`self.PatrolLoop`))

(event `PatrolLoop`
  ; Tree Patrolling
  (`|AIMoveTo` (`self.K2_GetPawn`) (`self.Tree Location`) null 100.0
    (:`OnSuccess`
      (if (`self.bIsPatrolling`)
        (`KismetSystemLibrary.Delay` 2.0)
        (`|AIMoveTo` (`self.K2_GetPawn`) (`self.Spawn Location`) null 100.0
          (:`OnSuccess`
            (`KismetSystemLibrary.Delay` 2.0)
            (`self.PatrolLoop`)))))))

(event `StartChase`
  (bind _returnvalue (`self.K2_GetPawn`))
  ; Chase to Player
  (set `self.OtherActing` true)
  (set `self.isChasing` true)
  (bind _asbp_ai_character (cast `/Game/Hide_easily/Blueprints/AI/BP_AI-Character` _returnvalue))
  (bind _chaseaudio (`/Game/Hide_easily/Blueprints/AI/BP_AI-Character.ChaseAudio` _asbp_ai_character))
  (`AudioComponent.Play` _chaseaudio 0.0)
  (bind _output_get (set `self.PlayerLocation` (`self.K2_GetActorLocation` (`GameplayStatics.GetPlayerPawn` 0))))
  (`|AIMoveTo` _returnvalue _output_get null 50.0
    (:`OnSuccess`
      (`KismetSystemLibrary.PrintString` "성공"))
    (:`OnFail`
      (`KismetSystemLibrary.PrintString` "실패")))
  (`AudioComponent.Stop` _chaseaudio)
  (set `self.OtherActing` false)
  (set `self.isChasing` false))

(event `SetInitialLocation`
  ; Location 초기화
  (bind _asbp_ai_character (cast `/Game/Hide_easily/Blueprints/AI/BP_AI-Character` (`self.K2_GetPawn`)))
  (set `self.Spawn Location` (`self.K2_GetActorLocation`))
  (set `self.Tree Location` (`self.K2_GetActorLocation` (`/Game/Hide_easily/Blueprints/AI/BP_AI-Character.Tree` _asbp_ai_character))))

(event `self.ReceiveBeginPlay`)

(event `self.AIPerception.OnTargetPerceptionUpdated`
  (params (Actor :type "Actor Object Reference") (Stimulus :type "AIStimulus Structure"))
  (bind (_age _expirationage _strength _stimuluslocation _receiverlocation _tag _bsuccessfullysensed) (break `AIStimulus` Stimulus))
  (bind _returnvalue (`AIBlueprintHelperLibrary.GetBlackboard` null))
  ;[1 1 1] Chase/ AI sees you
  ;;[1 1 1] is controlled by hideEasily controller?
  (bind _asbi_hide_easily_control (cast `/Game/Hide_easily/Blueprints/GameModeAndController/BI_HideEasilyControl` (`Pawn.GetController` (`Actor.Instigator` Actor)))
    (:`then`
      (bind _is_hiding_ (`/Game/Hide_easily/Blueprints/GameModeAndController/BI_HideEasilyControl.BI Get Is Hiding` _asbi_hide_easily_control))
      (if _is_hiding_
        (`BlackboardComponent.SetValueAsBool` _returnvalue "CanSeePlayer" false) ; if you hide, it stops following you
        (else
          (bind _dead (`/Game/Hide_easily/Blueprints/GameModeAndController/BI_HideEasilyControl.BI Get Dead` _asbi_hide_easily_control))
          (if (and (not _dead) (<= (`KismetMathLibrary.Vector_Distance` _stimuluslocation _receiverlocation) (`/Game/Hide_easily/Blueprints/AI/BP_AI-Character.Min Player Distance to Chase` (`self.NPC Pawn`))))
            (if (`BlackboardComponent.GetValueAsBool` _returnvalue "CanSeePlayer")
              (`BlackboardComponent.SetValueAsBool` _returnvalue "CanSeePlayer" _bsuccessfullysensed) ; if you hide, it stops following you
              (if (== _bsuccessfullysensed true)
                (`BlackboardComponent.SetValueAsObject` _returnvalue "ChaseActor" Actor :!label _label) ; follow the new player
                (else
                  ;[1 0.04223 0] Comment
                  (`AIPerceptionComponent.ForgetAll` (`self.AIPerception`))))
              (else
                (`BlackboardComponent.SetValueAsBool` _returnvalue "CanSeePlayer" true)
                (set `self.ChasingPlayer` Actor)
                (goto _label)))
            (else
              ;[1 0.04223 0] Comment
              (`AIPerceptionComponent.ForgetAll` (`self.AIPerception`)))))))
    (:`CastFailed`
      ;[1 0.04223 0] Comment
      (`AIPerceptionComponent.ForgetAll` (`self.AIPerception`)))))

(event `self.ReceiveTick`
  (params (DeltaSeconds :type "Float (single-precision)"))
  (bind _isplayerloud (`/Game/KJH/Widgets/WBP_Voice.IsPlayerLoud` (`self.HUDRef`)))
  (`/Engine/EditorBlueprintResources/StandardMacros.IsValid` (`self.HUDRef`)
    (:`Is Valid`
      (if _isplayerloud
        (set `self.bIsPatrolling` false)
        (`KismetSystemLibrary.PrintString` (`KismetStringLibrary.Conv_BoolToString` _isplayerloud))
        (`self.GoToRoomDoor`)))))

(event `GoToRoomDoor`
  (bind _asbp_santa_character (cast `/Game/KJH/BP/BP_SantaCharacter` (`GameplayStatics.GetPlayerCharacter` 0)))
  (bind _outactors (`GameplayStatics.GetAllActorsWithTag` (`KismetStringLibrary.Conv_StringToName` (`KismetStringLibrary.Concat_StrStr` "Door_" (`|GetEnumeratorNameAsString` (`/Game/KJH/BP/BP_SantaCharacter.CurrentRoon` _asbp_santa_character))))))
  (if (> (`KismetArrayLibrary.Array_Length` _outactors) 0)
    (bind _asbp_ai_character (cast `/Game/Hide_easily/Blueprints/AI/BP_AI-Character` (`self.K2_GetPawn`)))
    (`|AIMoveTo` _asbp_ai_character (0.0 0.0 0.0) (`|GetArrayItem` _outactors))))

(fn `CanInteractWithCloset?`
  (params (Key :type "Vector Structure (by ref)"))
  (returns (ReturnValue :type Boolean))
  (bind _patrolpath (`/Game/Hide_easily/Blueprints/AI/BP_AI-Character.PatrolPath` (`self.NPC Pawn`)))
  (return (`.ReturnValue` (`BlueprintMapLibrary.Map_Find` (`/Game/Hide_easily/Blueprints/AI/BP_PatrolPathAndClosets.LocationsForClosets` _patrolpath) (`KismetMathLibrary.InverseTransformLocation` (`self.GetTransform` _patrolpath) Key)))))

(fn `CloseClosetDoors`
  (params (Key :type "Vector Structure (by ref)"))
  (bind _patrolpath (`/Game/Hide_easily/Blueprints/AI/BP_AI-Character.PatrolPath` (`self.NPC Pawn`)))
  (bind (_value _returnvalue) (`BlueprintMapLibrary.Map_Find` (`/Game/Hide_easily/Blueprints/AI/BP_PatrolPathAndClosets.LocationsForClosets` _patrolpath) (`KismetMathLibrary.InverseTransformLocation` (`self.GetTransform` _patrolpath) Key)))
  (if _returnvalue
    (bind _asbp_closet_1 (cast `/Game/Hide_easily/Blueprints/BP_Closet_1` _value)
      (:`then`
        (`/Game/Hide_easily/Blueprints/BP_Closet_1.CloseDoors` _asbp_closet_1))
      (:`CastFailed`
        (bind _asbp_bed (cast `/Game/Hide_easily/Blueprints/BP_Bed` _value))
        (`/Game/Hide_easily/Blueprints/BP_Bed.CheckBedEnd` _asbp_bed)))))

(fn `IsSomeoaneInCloset?`
  (params (Location :type "Vector Structure"))
  (returns (Ocupied :type Boolean) (`Open doors` :type Boolean) (`Chasing Player` :type "Actor Object Reference"))
  (bind _patrolpath (`/Game/Hide_easily/Blueprints/AI/BP_AI-Character.PatrolPath` (`self.NPC Pawn`)))
  (bind (_value _returnvalue) (`BlueprintMapLibrary.Map_Find` (`/Game/Hide_easily/Blueprints/AI/BP_PatrolPathAndClosets.LocationsForClosets` _patrolpath) (`KismetMathLibrary.InverseTransformLocation` (`self.GetTransform` _patrolpath) Location)))
  (if _returnvalue
    (bind _asbp_closet_1 (cast `/Game/Hide_easily/Blueprints/BP_Closet_1` _value))
    (return (`KismetSystemLibrary.IsValid` (`/Game/Hide_easily/Blueprints/BP_Closet_1.UsingPlayer` _asbp_closet_1)) true null)
    (else
      (bind _asbp_bed (cast `/Game/Hide_easily/Blueprints/BP_Bed` _value))
      (return false false (`/Game/Hide_easily/Blueprints/BP_Bed.UsingPlayer` _asbp_bed)))))

(fn `OpenClosetDoors`
  (params (Key :type "Vector Structure (by ref)"))
  (bind _patrolpath (`/Game/Hide_easily/Blueprints/AI/BP_AI-Character.PatrolPath` (`self.NPC Pawn`)))
  (bind (_value _returnvalue) (`BlueprintMapLibrary.Map_Find` (`/Game/Hide_easily/Blueprints/AI/BP_PatrolPathAndClosets.LocationsForClosets` _patrolpath) (`KismetMathLibrary.InverseTransformLocation` (`self.GetTransform` _patrolpath) Key)))
  (if _returnvalue
    (bind _asbp_closet_1 (cast `/Game/Hide_easily/Blueprints/BP_Closet_1` _value)
      (:`then`
        (`/Game/Hide_easily/Blueprints/BP_Closet_1.OpenDoors` _asbp_closet_1))
      (:`CastFailed`
        (bind _asbp_bed (cast `/Game/Hide_easily/Blueprints/BP_Bed` _value))
        (`/Game/Hide_easily/Blueprints/BP_Bed.CheckBed` _asbp_bed)))))

(fn `UserConstructionScript`)