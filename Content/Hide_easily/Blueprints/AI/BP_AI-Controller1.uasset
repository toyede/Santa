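; AI controller for the hide-and-seek enemy in a Santa game, handling patrol, chase and closet/bed checks.
; Runs a behavior tree seeded from pawn settings; perception sets its chase keys for nearby, unhidden, living players.
; Event-driven phases also shuttle it between tree and spawn, switching to room-marker patrol when a present appears.
; Player noise, polled from the HUD during the first phase, sends it to that room's door; room investigation is stubbed.
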(event `StartPatrol`
  (set `self.bIsPatrolling` true)
  (`self.PatrolLoop`))

(event `PatrolLoop`
  ; Tree Patrolling
  (`|AIMoveTo` (`self.K2_GetPawn`) (`self.Tree Location`) null 100.0
    (:`OnSuccess`
      (if (`self.bIsPatrolling`)
        (`KismetSystemLibrary.Delay` 2.0)
        (`|AIMoveTo` (`self.K2_GetPawn`) (`self.Spawn Location`) null 100.0
          (:`OnSuccess`
            (`KismetSystemLibrary.Delay` 2.0)
            (`self.PatrolLoop`)))))))

(event `self.AIPerception.OnTargetPerceptionUpdated`
  (params (Actor :type "Actor Object Reference") (Stimulus :type "AIStimulus Structure"))
  (bind (_age _expirationage _strength _stimuluslocation _receiverlocation _tag _bsuccessfullysensed) (break `AIStimulus` Stimulus))
  (bind _returnvalue (`AIBlueprintHelperLibrary.GetBlackboard` null))
  ;[1 1 1] Chase/ AI sees you
  ;;[1 1 1] is controlled by hideEasily controller?
  (bind _asbi_hide_easily_control (cast `/Game/Hide_easily/Blueprints/GameModeAndController/BI_HideEasilyControl` (`Pawn.GetController` (`Actor.Instigator` Actor)))
    (:`then`
      (bind _is_hiding_ (`/Game/Hide_easily/Blueprints/GameModeAndController/BI_HideEasilyControl.BI Get Is Hiding` _asbi_hide_easily_control))
      (if _is_hiding_
        (`BlackboardComponent.SetValueAsBool` _returnvalue "CanSeePlayer" false) ; if you hide, it stops following you
        (else
          (bind _dead (`/Game/Hide_easily/Blueprints/GameModeAndController/BI_HideEasilyControl.BI Get Dead` _asbi_hide_easily_control))
          (if (and (not _dead) (<= (`KismetMathLibrary.Vector_Distance` _stimuluslocation _receiverlocation) (`/Game/Hide_easily/Blueprints/AI/BP_AI-Character.Min Player Distance to Chase` (`self.NPC Pawn`))))
            (if (`BlackboardComponent.GetValueAsBool` _returnvalue "CanSeePlayer")
              (`BlackboardComponent.SetValueAsBool` _returnvalue "CanSeePlayer" _bsuccessfullysensed) ; if you hide, it stops following you
              (if (== _bsuccessfullysensed true)
                (`BlackboardComponent.SetValueAsObject` _returnvalue "ChaseActor" Actor :!label _label) ; follow the new player
                (else
                  ;[1 0.04223 0] Comment
                  (`AIPerceptionComponent.ForgetAll` (`self.AIPerception`))))
              (else
                (`BlackboardComponent.SetValueAsBool` _returnvalue "CanSeePlayer" true)
                (set `self.ChasingPlayer` Actor)
                (goto _label)))
            (else
              ;[1 0.04223 0] Comment
              (`AIPerceptionComponent.ForgetAll` (`self.AIPerception`)))))))
    (:`CastFailed`
      ;[1 0.04223 0] Comment
      (`AIPerceptionComponent.ForgetAll` (`self.AIPerception`)))))

(event `self.ReceiveBeginPlay`
  (bind _returnvalue (`AIBlueprintHelperLibrary.GetBlackboard` null))
  ; BeginPlay
  (`KismetSystemLibrary.Delay` 0.5)
  (bind _asbp_santa_controller_1 (cast `/Game/KSH/BP/BP_SantaController1` (`GameplayStatics.GetPlayerController` 0)))
  (set `self.HUDRef` (`/Game/KSH/BP/BP_SantaController1.HUDRef` _asbp_santa_controller_1))
  (set `self.PlayerPawn` (`GameplayStatics.GetPlayerPawn` 0))
  (bind _outactors (`GameplayStatics.GetAllActorsOfClass` "/Game/KSH/Tree.Tree_C"))
  (set `self.TreeActorRef` (`|GetArrayItem` _outactors))
  (set `self.Phase` "NewEnumerator0")
  (set `self.bIsPlayerLoudPreviously ` false)
  (`self.SetInitialLocation`)
  (set `self.bIsPatrollingPhase1` true)
  (`self.PatrolPhase1`)
  (bind _outactors_2 (`GameplayStatics.GetAllActorsWithTag` "Marker"))
  (bind _output_get (set `self.ParolRoomMarkers` _outactors_2))
  (`KismetSystemLibrary.PrintString` (`KismetStringLibrary.Conv_IntToString` (`KismetArrayLibrary.Array_Length` _output_get)))
  (set `self.PlayerCurrentRoom` "NewEnumerator0")
  (set `self.LastTargetRoom` "NewEnumerator0")
  (set `self.PatrolRoomIndex` 0)
  (set `self.bIsPatrollingPhase2` false)
  (`self.RunBehaviorTree` "/Game/Hide_easily/Blueprints/AI/BT_PatrolChaseAndSearch.BT_PatrolChaseAndSearch")
  (bind _asbp_ai_character (cast `/Game/Hide_easily/Blueprints/AI/BP_AI-Character` (`self.K2_GetPawn`)))
  (set `self.NPC Pawn` _asbp_ai_character)
  (`BlackboardComponent.SetValueAsFloat` _returnvalue "Time" (`/Game/Hide_easily/Blueprints/AI/BP_AI-Character.Wait Time` (`self.NPC Pawn`)))
  (`BlackboardComponent.SetValueAsBool` _returnvalue "PathLoop" (`/Game/Hide_easily/Blueprints/AI/BP_AI-Character.Is Looping?` (`self.NPC Pawn`)))
  (`BlackboardComponent.SetValueAsInt` _returnvalue "Direction" 1)
  (`BlackboardComponent.SetValueAsFloat` _returnvalue "PatrolSpeed" (`/Game/Hide_easily/Blueprints/AI/BP_AI-Character.Patrol Speed` (`self.NPC Pawn`)))
  (`BlackboardComponent.SetValueAsFloat` _returnvalue "ChaseSpeed" (`/Game/Hide_easily/Blueprints/AI/BP_AI-Character.Chase Speed` (`self.NPC Pawn`)))
  (`BlackboardComponent.SetValueAsFloat` _returnvalue "MinDistanceToAttack" (`/Game/Hide_easily/Blueprints/AI/BP_AI-Character.Min Player Distance to Attack` (`self.NPC Pawn`)))
  (`BlackboardComponent.SetValueAsFloat` _returnvalue "MinDistanceToChase" (`/Game/Hide_easily/Blueprints/AI/BP_AI-Character.Min Player Distance to Chase` (`self.NPC Pawn`)))
  (`BlackboardComponent.SetValueAsBool` _returnvalue "KillPlayers?" (`/Game/Hide_easily/Blueprints/AI/BP_AI-Character.Kill Players?` (`self.NPC Pawn`))))

(event `RoomPatrol`
  (set `self.IsRoomPatroling` true)
  (if (> (`KismetArrayLibrary.Array_Length` (`self.ParolRoomMarkers`)) 0)
    (`|AIMoveTo` (`self.K2_GetPawn`) (0.0 0.0 0.0) null)))

(event `SetInitialLocation`
  ; Location 초기화
  (bind _asbp_ai_character (cast `/Game/Hide_easily/Blueprints/AI/BP_AI-Character` (`self.K2_GetPawn`)))
  (set `self.Spawn Location` (`self.K2_GetActorLocation`))
  (set `self.Tree Location` (`self.K2_GetActorLocation` (`/Game/Hide_easily/Blueprints/AI/BP_AI-Character.Tree` _asbp_ai_character))))

(event `StartPhase2`
  ; StartPhase2
  (set `self.Phase` "NewEnumerator5")
  (set `self.bIsPatrollingPhase2` true)
  (set `self.PatrolRoomIndex` 0)
  (`KismetSystemLibrary.PrintString` (`|GetEnumeratorNameAsString` (`self.Phase`)))
  (`self.PatrolPhase2`))

(event `PatrolPhase2`
  ; PatrolPhase2
  (if (and (`|EnumEquality` (`self.Phase`) "NewEnumerator5") (`self.bIsPatrollingPhase2`))
    (`KismetSystemLibrary.PrintString` "2페입갤")
    (if (> (`KismetArrayLibrary.Array_Length` (`self.ParolRoomMarkers`)) 0)
      (`KismetSystemLibrary.PrintString` "룸마커 길이 > 0")
      (bind _output_get (set `self.CurrentRoomMarker` (`|GetArrayItem` (`self.ParolRoomMarkers`) (`self.PatrolRoomIndex`))))
      (`|AIMoveTo` (`self.K2_GetPawn`) (0.0 0.0 0.0) _output_get 50.0
        (:`OnSuccess`
          (set `self.PatrolRoomIndex` (mod (+ (`self.PatrolRoomIndex`) 1) (`KismetArrayLibrary.Array_Length` (`self.ParolRoomMarkers`))))
          (`KismetSystemLibrary.Delay` 1.0))
        (:`OnFail`
          _))
      (`self.PatrolPhase2`))))

(event `PatrolPhase1`
  ; PatrolPhase1
  (if (and (`|EnumEquality` (`self.Phase`) "NewEnumerator0") (`self.bIsPatrollingPhase1`))
    (`|AIMoveTo` (`self.K2_GetPawn`) (`self.Tree Location`) null 100.0
      (:`OnSuccess`
        (`self.AfterArriveTree`))
      (:`OnFail`
        (`KismetSystemLibrary.Delay` 1.0)
        (`self.PatrolPhase1`)))))

(event `AfterArriveTree`
  ; AfterArriveTree
  (if (and (`|EnumEquality` (`self.Phase`) "NewEnumerator0") (`self.bIsPatrollingPhase1`))
    (bind _output_get (set `self.bExist` (`/Game/KSH/Tree.IsExistPresent` (`self.TreeActorRef`))))
    (if _output_get
      (set `self.Phase` "NewEnumerator5")
      (set `self.bIsPatrollingPhase1` false)
      (`self.StartPhase2`)
      (else
        (`KismetSystemLibrary.Delay` 1.0)
        (`self.MoveSpawnLocation`)))))

(event `InvestigateMarkerPhase2`
  (if (and (`|EnumEquality` (`self.Phase`) "NewEnumerator5") (`self.bIsPatrollingPhase2`))
    (switch `string` (`KismetStringLibrary.GetSubstring` (`KismetSystemLibrary.GetDisplayName` (`self.CurrentRoomMarker`)) 7)
      (:`Room_A`
        (set `self.ThisRoomID` "NewEnumerator1"))
      (:`Room_B`
        (set `self.ThisRoomID` "NewEnumerator2"))
      (:`Room_C`
        (set `self.ThisRoomID` "NewEnumerator3"))
      (:`Room_D`
        (set `self.ThisRoomID` "NewEnumerator4"))
      (:`Room_E`
        (set `self.ThisRoomID` "NewEnumerator5")))
    (if (`|EnumEquality` (`self.PlayerCurrentRoom`) (`self.ThisRoomID`))
      (`self.InvestigatePlayerInRoomPhase2`)
      (else
        (`self.InvestigateRoomStructuresPhase2`)))))

(event `MoveSpawnLocation`
  ; MoveSpawnLocation
  (if (and (`|EnumEquality` (`self.Phase`) "NewEnumerator0") (`self.bIsPatrollingPhase1`))
    (`|AIMoveTo` (`self.K2_GetPawn`) (`self.Spawn Location`) null 100.0
      (:`OnSuccess`
        (`self.AfterArriveSpawn`))
      (:`OnFail`
        (`KismetSystemLibrary.Delay` 1.0)
        (`self.PatrolPhase1`)))))

(event `AfterArriveSpawn`
  ; AfterArriveSpawn
  (if (and (`|EnumEquality` (`self.Phase`) "NewEnumerator0") (`self.bIsPatrollingPhase1`))
    (bind _output_get (set `self.bExist` (`/Game/KSH/Tree.IsExistPresent` (`self.TreeActorRef`))))
    (if _output_get
      (set `self.Phase` "NewEnumerator5")
      (set `self.bIsPatrollingPhase1` false)
      (`self.StartPhase2`)
      (else
        (`KismetSystemLibrary.Delay` 1.0)
        (`self.PatrolPhase1`)))))

(event `self.ReceiveTick`
  (params (DeltaSeconds :type "Float (single-precision)"))
  ; Tick
  (`/Engine/EditorBlueprintResources/StandardMacros.IsValid` (`self.HUDRef`)
    (:`Is Valid`
      (set `self.bIsPlayerLoud` (`/Game/KJH/Widgets/WBP_Voice.IsPlayerLoud` (`self.HUDRef`)))
      (if (and (`self.bIsPlayerLoud`) (== (`self.bIsPlayerLoudPreviously `) false))
        (if (and (`|EnumEquality` (`self.Phase`) "NewEnumerator0") (`self.bIsPatrollingPhase1`))
          (set `self.bIsPatrollingPhase1` false)
          (set `self.Phase` "NewEnumerator1")
          (`KismetSystemLibrary.PrintString` "감지!")
          (`KismetSystemLibrary.PrintString` (`KismetSystemLibrary.GetDisplayName` (`self.CurrentRoomMarker`)))
          (`self.StartChase`)
          (set `self.bIsPlayerLoudPreviously ` (`self.bIsPlayerLoud`)))))))

(event `InvestigatePlayerInRoomPhase2`)

(event `InvestigateRoomStructuresPhase2`
  (if (== (`|EnumEquality` (`self.Phase`) "NewEnumerator5") (`self.bIsPatrollingPhase2`))
    (switch `string` (`KismetStringLibrary.GetSubstring` (`KismetSystemLibrary.GetDisplayName` (`self.CurrentRoomMarker`)) 7)
      (:`Room_A`
        (set `self.ThisRoomID` "NewEnumerator1"))
      (:`Room_B`
        (set `self.ThisRoomID` "NewEnumerator2"))
      (:`Room_C`
        (set `self.ThisRoomID` "NewEnumerator3"))
      (:`Room_D`
        (set `self.ThisRoomID` "NewEnumerator4"))
      (:`Room_E`
        (set `self.ThisRoomID` "NewEnumerator5")))
    (bind _outactors (`GameplayStatics.GetAllActorsWithTag` (`KismetStringLibrary.Conv_StringToName` (`KismetStringLibrary.Concat_StrStr` "Structure_" (`|GetEnumeratorNameAsString` (`self.ThisRoomID`))))))
    (if (> (`KismetArrayLibrary.Array_Length` _outactors) 0)
      (for _ _outactors
        _)
      (`self.ContinuePhase2`)
      (else
        (`self.ContinuePhase2`)))))

(event `StartChase`
  ; StartChase
  (if (`|EnumEquality` (`self.Phase`) "NewEnumerator1")
    (`self.GoToRoomDoor`)))

(event `ContinuePhase2`)

(event `GoToRoomDoor`
  ; GoToRoomDoor
  (bind _asbp_santa_character (cast `/Game/KJH/BP/BP_SantaCharacter` (`GameplayStatics.GetPlayerCharacter` 0)))
  (set `self.PlayerCurrentRoom` (`/Game/KJH/BP/BP_SantaCharacter.CurrentRoon` _asbp_santa_character))
  (if (not (or (`|EnumEquality` (`self.PlayerCurrentRoom`) "NewEnumerator0") (`|EnumEquality` (`self.PlayerCurrentRoom`) (`self.LastTargetRoom`))))
    (bind _outactors (`GameplayStatics.GetAllActorsWithTag` (`KismetStringLibrary.Conv_StringToName` (`KismetStringLibrary.Concat_StrStr` "Door_" (`|GetEnumeratorNameAsString` (`/Game/KJH/BP/BP_SantaCharacter.CurrentRoon` _asbp_santa_character))))))
    (if (> (`KismetArrayLibrary.Array_Length` _outactors) 0)
      (bind _asbp_ai_character (cast `/Game/Hide_easily/Blueprints/AI/BP_AI-Character` (`self.K2_GetPawn`)))
      (`|AIMoveTo` _asbp_ai_character (0.0 0.0 0.0) (`|GetArrayItem` _outactors) 30.0
        (:`OnSuccess`
          (`KismetSystemLibrary.PrintString` "도착은 함")
          (`self.StartPhase2`))))))

(fn `CanInteractWithCloset?`
  (params (Key :type "Vector Structure (by ref)"))
  (returns (ReturnValue :type Boolean))
  (bind _patrolpath (`/Game/Hide_easily/Blueprints/AI/BP_AI-Character.PatrolPath` (`self.NPC Pawn`)))
  (return (`.ReturnValue` (`BlueprintMapLibrary.Map_Find` (`/Game/Hide_easily/Blueprints/AI/BP_PatrolPathAndClosets.LocationsForClosets` _patrolpath) (`KismetMathLibrary.InverseTransformLocation` (`self.GetTransform` _patrolpath) Key)))))

(fn `CloseClosetDoors`
  (params (Key :type "Vector Structure (by ref)"))
  (bind _patrolpath (`/Game/Hide_easily/Blueprints/AI/BP_AI-Character.PatrolPath` (`self.NPC Pawn`)))
  (bind (_value _returnvalue) (`BlueprintMapLibrary.Map_Find` (`/Game/Hide_easily/Blueprints/AI/BP_PatrolPathAndClosets.LocationsForClosets` _patrolpath) (`KismetMathLibrary.InverseTransformLocation` (`self.GetTransform` _patrolpath) Key)))
  (if _returnvalue
    (bind _asbp_closet_1 (cast `/Game/Hide_easily/Blueprints/BP_Closet_1` _value)
      (:`then`
        (`/Game/Hide_easily/Blueprints/BP_Closet_1.CloseDoors` _asbp_closet_1))
      (:`CastFailed`
        (bind _asbp_bed (cast `/Game/Hide_easily/Blueprints/BP_Bed` _value))
        (`/Game/Hide_easily/Blueprints/BP_Bed.CheckBedEnd` _asbp_bed)))))

(fn `IsSomeoaneInCloset?`
  (params (Location :type "Vector Structure"))
  (returns (Ocupied :type Boolean) (`Open doors` :type Boolean) (`Chasing Player` :type "Actor Object Reference"))
  (bind _patrolpath (`/Game/Hide_easily/Blueprints/AI/BP_AI-Character.PatrolPath` (`self.NPC Pawn`)))
  (bind (_value _returnvalue) (`BlueprintMapLibrary.Map_Find` (`/Game/Hide_easily/Blueprints/AI/BP_PatrolPathAndClosets.LocationsForClosets` _patrolpath) (`KismetMathLibrary.InverseTransformLocation` (`self.GetTransform` _patrolpath) Location)))
  (if _returnvalue
    (bind _asbp_closet_1 (cast `/Game/Hide_easily/Blueprints/BP_Closet_1` _value))
    (return (`KismetSystemLibrary.IsValid` (`/Game/Hide_easily/Blueprints/BP_Closet_1.UsingPlayer` _asbp_closet_1)) true null)
    (else
      (bind _asbp_bed (cast `/Game/Hide_easily/Blueprints/BP_Bed` _value))
      (return false false (`/Game/Hide_easily/Blueprints/BP_Bed.UsingPlayer` _asbp_bed)))))

(fn `OpenClosetDoors`
  (params (Key :type "Vector Structure (by ref)"))
  (bind _patrolpath (`/Game/Hide_easily/Blueprints/AI/BP_AI-Character.PatrolPath` (`self.NPC Pawn`)))
  (bind (_value _returnvalue) (`BlueprintMapLibrary.Map_Find` (`/Game/Hide_easily/Blueprints/AI/BP_PatrolPathAndClosets.LocationsForClosets` _patrolpath) (`KismetMathLibrary.InverseTransformLocation` (`self.GetTransform` _patrolpath) Key)))
  (if _returnvalue
    (bind _asbp_closet_1 (cast `/Game/Hide_easily/Blueprints/BP_Closet_1` _value)
      (:`then`
        (`/Game/Hide_easily/Blueprints/BP_Closet_1.OpenDoors` _asbp_closet_1))
      (:`CastFailed`
        (bind _asbp_bed (cast `/Game/Hide_easily/Blueprints/BP_Bed` _value))
        (`/Game/Hide_easily/Blueprints/BP_Bed.CheckBed` _asbp_bed)))))

(fn `UserConstructionScript`)