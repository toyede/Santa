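; BP_WC is a toilet-themed hiding spot that specializes a parent hideable, destroying the right-door components and left knob to leave a single swinging door.
; It overrides the door open/close with a timeline rotating the left door, whose length and curve follow the hide speed.
; Hide drives the player controller through BI_HideEasilyControl: lock input, optionally face the door, move the pawn inside, then close up, using speed-based delays.
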(event `self.OpenDoors`
  ;[1 1 1] OPEN/CLOSE DORS  overwrite
  (bind (_direction _track_0) (`Timeline|New Open/Close Doors` :!label _label)
    (:`Update`
      (`SceneComponent.K2_SetRelativeRotation` (`self.LeftDoorRoot`) (`KismetMathLibrary.RLerp` (struct :`Pitch` 90.0 :`Yaw` 180.0 :`Roll` 180.0) (struct :`Pitch` 90.0 :`Yaw` -65.0 :`Roll` 180.0) _track_0 true) false false))))

(event `self.CloseDoors`
  ;[1 1 1] OPEN/CLOSE DORS  overwrite
  (goto _label :!via `Reverse`))

(event `self.Hide`
  (params (Pawn :type "Actor Object Reference") (PlayerController :type "PlayerController Object Reference"))
  (bind _asbi_hide_easily_control (cast `/Game/Hide_easily/Blueprints/GameModeAndController/BI_HideEasilyControl` PlayerController :!pure true))
  (bind _hidespeed (`self.HideSpeed`))
  (bind _value (`BlueprintMapLibrary.Map_Find` (`self.Delays`) _hidespeed))
  (bind _returnvalue (`SceneComponent.K2_GetComponentLocation` (`Actor.RootComponent` Pawn)))
  (bind _returnvalue_2 (+ _value 0.2))
  ;[1 0.1108 0] change original delay
  (`/Game/Hide_easily/Blueprints/GameModeAndController/BI_HideEasilyControl.BI Update Hiding` _asbi_hide_easily_control "true")
  (`/Game/Hide_easily/Blueprints/GameModeAndController/BI_HideEasilyControl.BI Disable Player Input` _asbi_hide_easily_control)
  (set `self.Hiding` true)
  (`self.Server_Hide_Message` _asbi_hide_easily_control)
  ;[1 1 1] Rotate
  (if (`self.RotateBeforeHide`)
    (`/Game/Hide_easily/Blueprints/GameModeAndController/BI_HideEasilyControl.BI Rotate To Face Doors` _asbi_hide_easily_control Pawn _returnvalue (`SceneComponent.K2_GetComponentLocation` (`self.Location_In`)))
    (`KismetSystemLibrary.Delay` 0.2))
  (`self.OpenDoors`)
  (`KismetSystemLibrary.Delay` _value)
  (`/Game/Hide_easily/Blueprints/GameModeAndController/BI_HideEasilyControl.BI Player Go In` _asbi_hide_easily_control _returnvalue (`SceneComponent.K2_GetComponentLocation` (`self.Location_In`)) Pawn _hidespeed (`self.RotateWhenHide`))
  (`KismetSystemLibrary.Delay` _returnvalue_2)
  (`self.CloseDoors`)
  (`KismetSystemLibrary.Delay` (+ _returnvalue_2 0.3)) ; wait until you get inside
  (`self.Server_Show_Message` _asbi_hide_easily_control) ; enable unhide
  (set `self.Hiding` false)
  (`/Game/Hide_easily/Blueprints/GameModeAndController/BI_HideEasilyControl.BI Update Hiding` _asbi_hide_easily_control false))

(fn `SetHideSpeed`
  (bind _new_open_close_doors (`self.New Open/Close Doors`))
  (bind _hidespeed (`self.HideSpeed`))
  (`TimelineComponent.SetTimelineLength` _new_open_close_doors (select `/Game/Hide_easily/Blueprints/GameModeAndController/E_HideSpeed` _hidespeed :`NewEnumerator0` 0.7 :`NewEnumerator1` 0.5 :!type "Float (single-precision)"))
  (`TimelineComponent.SetFloatCurve` _new_open_close_doors (select `/Game/Hide_easily/Blueprints/GameModeAndController/E_HideSpeed` _hidespeed :`NewEnumerator0` "/Game/Hide_easily/Curves/C_Point7.C_Point7" :`NewEnumerator1` "/Game/Hide_easily/Curves/C_Point5.C_Point5" :!type "CurveFloat Object Reference") "Track_0"))

(fn `UserConstructionScript`
  (`parent.UserConstructionScript`)
  (`ActorComponent.K2_DestroyComponent` (`self.RightDoorRoot`))
  (`ActorComponent.K2_DestroyComponent` (`self.LeftDoorknob`))
  (`ActorComponent.K2_DestroyComponent` (`self.RightDoorMesh`))
  (`ActorComponent.K2_DestroyComponent` (`self.RightDoorknob`)))